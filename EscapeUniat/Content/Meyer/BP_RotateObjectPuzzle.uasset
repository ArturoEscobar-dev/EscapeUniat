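; Four-object rotation puzzle that the player solves by turning each object into place, currently only printing a success message.
; Player trigger volumes enable input and open a per-object gate, so Interact yaws that object by AngleRotation through a timeline, with input disabled during the turn.
; Puzzle triggers set each object's flag while overlapping a BP_RotateObjectivePuzzle actor.
; A looping timer polls all four flags to detect the solved state.
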(event `self.ReceiveBeginPlay`
  (`|ExecutionSequence`
    (:`then_0`
      (set `self.CurrentRotationObjectOne` (`SceneComponent.K2_GetComponentRotation` (`self.ObjectOne`)))
      (set `self.CurrentRotationObjectTwo` (`SceneComponent.K2_GetComponentRotation` (`self.ObjectTwo`)))
      (set `self.CurrentRotationObjectThree` (`SceneComponent.K2_GetComponentRotation` (`self.ObjectThree`)))
      (set `self.CurrentRotationObjectFour` (`SceneComponent.K2_GetComponentRotation` (`self.ObjectFour`))))
    (:`then_1`
      (`KismetSystemLibrary.K2_SetTimer` null "PuzzleResolved" 0.25 true))))

(event `PuzzleResolved`
  (if (and (and (`self.ObjectOneActivate`) (`self.ObjectTwoActivate`)) (and (`self.ObjectThreeActivate`) (`self.ObjectFourActivate`)))
    (`KismetSystemLibrary.PrintString` "Puzzle Correcto")))

(event `EnhancedInput|/Game/ThirdPerson/Input/Actions/IA_Interact`
  (params (ActionValue :type Boolean) (ElapsedSeconds :type "Float (double-precision)") (TriggeredSeconds :type "Float (double-precision)") (InputAction :type "InputAction Object Reference" :default "/Game/ThirdPerson/Input/Actions/IA_Interact.IA_Interact"))
  (bind _currentrotationobjectone (`self.CurrentRotationObjectOne`))
  (:`Triggered`
    (`/Engine/EditorBlueprintResources/StandardMacros.Gate` true :!label _label
      (:`Exit`
        (`self.DisableInput` (`GameplayStatics.GetPlayerController` 0))
        (bind (_direction _newtrack_0) (`Timeline|TimelineObjectOne` :!via `PlayFromStart`)
          (:`Update`
            (bind _returnvalue (`KismetMathLibrary.RLerp` _currentrotationobjectone (`KismetMathLibrary.MakeRotator` (.roll _currentrotationobjectone) (.pitch _currentrotationobjectone) (+ (.yaw _currentrotationobjectone) (`self.AngleRotation`))) _newtrack_0))
            (`SceneComponent.K2_SetRelativeRotation` (`self.ObjectOne`) _returnvalue false false))
          (:`Finished`
            (set `self.CurrentRotationObjectOne` _returnvalue)
            (`self.EnableInput` (`GameplayStatics.GetPlayerController` 0))))))))

(event `self.TriggerObjectOne.OnComponentBeginOverlap`
  (params (OverlappedComponent :type "PrimitiveComponent Object Reference") (OtherActor :type "Actor Object Reference") (OtherComp :type "PrimitiveComponent Object Reference") (OtherBodyIndex :type Integer) (bFromSweep :type Boolean) (SweepResult :type "HitResult Structure (by ref)"))
  (cast `/Game/ThirdPerson/Blueprints/BP_PlayerCharacter` OtherActor)
  (`self.EnableInput` (`GameplayStatics.GetPlayerController` 0))
  (goto _label :!via `Open`))

(event `self.TriggerObjectOne.OnComponentEndOverlap`
  (params (OverlappedComponent :type "PrimitiveComponent Object Reference") (OtherActor :type "Actor Object Reference") (OtherComp :type "PrimitiveComponent Object Reference") (OtherBodyIndex :type Integer))
  (cast `/Game/ThirdPerson/Blueprints/BP_PlayerCharacter` OtherActor)
  (`self.DisableInput` (`GameplayStatics.GetPlayerController` 0))
  (goto _label :!via `Close`))

(event `self.TriggerPuzzleOne.OnComponentBeginOverlap`
  (params (OverlappedComponent :type "PrimitiveComponent Object Reference") (OtherActor :type "Actor Object Reference") (OtherComp :type "PrimitiveComponent Object Reference") (OtherBodyIndex :type Integer) (bFromSweep :type Boolean) (SweepResult :type "HitResult Structure (by ref)"))
  (cast `/Game/Meyer/BP_RotateObjectivePuzzle` OtherActor)
  (set `self.ObjectOneActivate` true))

(event `self.TriggerPuzzleOne.OnComponentEndOverlap`
  (params (OverlappedComponent :type "PrimitiveComponent Object Reference") (OtherActor :type "Actor Object Reference") (OtherComp :type "PrimitiveComponent Object Reference") (OtherBodyIndex :type Integer))
  (cast `/Game/Meyer/BP_RotateObjectivePuzzle` OtherActor)
  (set `self.ObjectOneActivate` false))

(event `EnhancedInput|/Game/ThirdPerson/Input/Actions/IA_Interact`
  (params (ActionValue :type Boolean) (ElapsedSeconds :type "Float (double-precision)") (TriggeredSeconds :type "Float (double-precision)") (InputAction :type "InputAction Object Reference" :default "/Game/ThirdPerson/Input/Actions/IA_Interact.IA_Interact"))
  (bind _currentrotationobjecttwo (`self.CurrentRotationObjectTwo`))
  (:`Triggered`
    (`/Engine/EditorBlueprintResources/StandardMacros.Gate` true :!label _label_2
      (:`Exit`
        (`self.DisableInput` (`GameplayStatics.GetPlayerController` 0))
        (bind (_direction _newtrack_0) (`Timeline|Timeline` :!via `PlayFromStart`)
          (:`Update`
            (bind _returnvalue (`KismetMathLibrary.RLerp` _currentrotationobjecttwo (`KismetMathLibrary.MakeRotator` (.roll _currentrotationobjecttwo) (.pitch _currentrotationobjecttwo) (+ (.yaw _currentrotationobjecttwo) (`self.AngleRotation`))) _newtrack_0))
            (`SceneComponent.K2_SetRelativeRotation` (`self.ObjectTwo`) _returnvalue false false))
          (:`Finished`
            (set `self.CurrentRotationObjectTwo` _returnvalue)
            (`self.EnableInput` (`GameplayStatics.GetPlayerController` 0))))))))

(event `self.TriggerObjectTwo.OnComponentBeginOverlap`
  (params (OverlappedComponent :type "PrimitiveComponent Object Reference") (OtherActor :type "Actor Object Reference") (OtherComp :type "PrimitiveComponent Object Reference") (OtherBodyIndex :type Integer) (bFromSweep :type Boolean) (SweepResult :type "HitResult Structure (by ref)"))
  (cast `/Game/ThirdPerson/Blueprints/BP_PlayerCharacter` OtherActor)
  (`self.EnableInput` (`GameplayStatics.GetPlayerController` 0))
  (goto _label_2 :!via `Open`))

(event `self.TriggerObjectTwo.OnComponentEndOverlap`
  (params (OverlappedComponent :type "PrimitiveComponent Object Reference") (OtherActor :type "Actor Object Reference") (OtherComp :type "PrimitiveComponent Object Reference") (OtherBodyIndex :type Integer))
  (cast `/Game/ThirdPerson/Blueprints/BP_PlayerCharacter` OtherActor)
  (`self.DisableInput` (`GameplayStatics.GetPlayerController` 0))
  (goto _label_2 :!via `Close`))

(event `self.TriggerPuzzleTwo.OnComponentBeginOverlap`
  (params (OverlappedComponent :type "PrimitiveComponent Object Reference") (OtherActor :type "Actor Object Reference") (OtherComp :type "PrimitiveComponent Object Reference") (OtherBodyIndex :type Integer) (bFromSweep :type Boolean) (SweepResult :type "HitResult Structure (by ref)"))
  (cast `/Game/Meyer/BP_RotateObjectivePuzzle` OtherActor)
  (set `self.ObjectTwoActivate` true))

(event `self.TriggerPuzzleTwo.OnComponentEndOverlap`
  (params (OverlappedComponent :type "PrimitiveComponent Object Reference") (OtherActor :type "Actor Object Reference") (OtherComp :type "PrimitiveComponent Object Reference") (OtherBodyIndex :type Integer))
  (cast `/Game/Meyer/BP_RotateObjectivePuzzle` OtherActor)
  (set `self.ObjectTwoActivate` false))

(event `EnhancedInput|/Game/ThirdPerson/Input/Actions/IA_Interact`
  (params (ActionValue :type Boolean) (ElapsedSeconds :type "Float (double-precision)") (TriggeredSeconds :type "Float (double-precision)") (InputAction :type "InputAction Object Reference" :default "/Game/ThirdPerson/Input/Actions/IA_Interact.IA_Interact"))
  (bind _currentrotationobjectthree (`self.CurrentRotationObjectThree`))
  (:`Triggered`
    (`/Engine/EditorBlueprintResources/StandardMacros.Gate` true :!label _label_3
      (:`Exit`
        (`self.DisableInput` (`GameplayStatics.GetPlayerController` 0))
        (bind (_direction _newtrack_0) (`Timeline|Timeline_0` :!via `PlayFromStart`)
          (:`Update`
            (bind _returnvalue (`KismetMathLibrary.RLerp` _currentrotationobjectthree (`KismetMathLibrary.MakeRotator` (.roll _currentrotationobjectthree) (.pitch _currentrotationobjectthree) (+ (.yaw _currentrotationobjectthree) (`self.AngleRotation`))) _newtrack_0))
            (`SceneComponent.K2_SetRelativeRotation` (`self.ObjectThree`) _returnvalue false false))
          (:`Finished`
            (set `self.CurrentRotationObjectThree` _returnvalue)
            (`self.EnableInput` (`GameplayStatics.GetPlayerController` 0))))))))

(event `self.TriggerObjectThree.OnComponentBeginOverlap`
  (params (OverlappedComponent :type "PrimitiveComponent Object Reference") (OtherActor :type "Actor Object Reference") (OtherComp :type "PrimitiveComponent Object Reference") (OtherBodyIndex :type Integer) (bFromSweep :type Boolean) (SweepResult :type "HitResult Structure (by ref)"))
  (cast `/Game/ThirdPerson/Blueprints/BP_PlayerCharacter` OtherActor)
  (`self.EnableInput` (`GameplayStatics.GetPlayerController` 0))
  (goto _label_3 :!via `Open`))

(event `self.TriggerObjectThree.OnComponentEndOverlap`
  (params (OverlappedComponent :type "PrimitiveComponent Object Reference") (OtherActor :type "Actor Object Reference") (OtherComp :type "PrimitiveComponent Object Reference") (OtherBodyIndex :type Integer))
  (cast `/Game/ThirdPerson/Blueprints/BP_PlayerCharacter` OtherActor)
  (`self.DisableInput` (`GameplayStatics.GetPlayerController` 0))
  (goto _label_3 :!via `Close`))

(event `self.TriggerPuzzleThree.OnComponentBeginOverlap`
  (params (OverlappedComponent :type "PrimitiveComponent Object Reference") (OtherActor :type "Actor Object Reference") (OtherComp :type "PrimitiveComponent Object Reference") (OtherBodyIndex :type Integer) (bFromSweep :type Boolean) (SweepResult :type "HitResult Structure (by ref)"))
  (cast `/Game/Meyer/BP_RotateObjectivePuzzle` OtherActor)
  (set `self.ObjectThreeActivate` true))

(event `self.TriggerPuzzleThree.OnComponentEndOverlap`
  (params (OverlappedComponent :type "PrimitiveComponent Object Reference") (OtherActor :type "Actor Object Reference") (OtherComp :type "PrimitiveComponent Object Reference") (OtherBodyIndex :type Integer))
  (cast `/Game/Meyer/BP_RotateObjectivePuzzle` OtherActor)
  (set `self.ObjectThreeActivate` false))

(event `EnhancedInput|/Game/ThirdPerson/Input/Actions/IA_Interact`
  (params (ActionValue :type Boolean) (ElapsedSeconds :type "Float (double-precision)") (TriggeredSeconds :type "Float (double-precision)") (InputAction :type "InputAction Object Reference" :default "/Game/ThirdPerson/Input/Actions/IA_Interact.IA_Interact"))
  (bind _currentrotationobjectfour (`self.CurrentRotationObjectFour`))
  (:`Triggered`
    (`/Engine/EditorBlueprintResources/StandardMacros.Gate` true :!label _label_4
      (:`Exit`
        (`self.DisableInput` (`GameplayStatics.GetPlayerController` 0))
        (bind (_direction _newtrack_0) (`Timeline|Timeline_1` :!via `PlayFromStart`)
          (:`Update`
            (bind _returnvalue (`KismetMathLibrary.RLerp` _currentrotationobjectfour (`KismetMathLibrary.MakeRotator` (.roll _currentrotationobjectfour) (.pitch _currentrotationobjectfour) (+ (.yaw _currentrotationobjectfour) (`self.AngleRotation`))) _newtrack_0))
            (`SceneComponent.K2_SetRelativeRotation` (`self.ObjectFour`) _returnvalue false false))
          (:`Finished`
            (set `self.CurrentRotationObjectFour` _returnvalue)
            (`self.EnableInput` (`GameplayStatics.GetPlayerController` 0))))))))

(event `self.TriggerObjectFour.OnComponentBeginOverlap`
  (params (OverlappedComponent :type "PrimitiveComponent Object Reference") (OtherActor :type "Actor Object Reference") (OtherComp :type "PrimitiveComponent Object Reference") (OtherBodyIndex :type Integer) (bFromSweep :type Boolean) (SweepResult :type "HitResult Structure (by ref)"))
  (cast `/Game/ThirdPerson/Blueprints/BP_PlayerCharacter` OtherActor)
  (`self.EnableInput` (`GameplayStatics.GetPlayerController` 0))
  (goto _label_4 :!via `Open`))

(event `self.TriggerObjectFour.OnComponentEndOverlap`
  (params (OverlappedComponent :type "PrimitiveComponent Object Reference") (OtherActor :type "Actor Object Reference") (OtherComp :type "PrimitiveComponent Object Reference") (OtherBodyIndex :type Integer))
  (cast `/Game/ThirdPerson/Blueprints/BP_PlayerCharacter` OtherActor)
  (`self.DisableInput` (`GameplayStatics.GetPlayerController` 0))
  (goto _label_4 :!via `Close`))

(event `self.TriggerPuzzleFour.OnComponentBeginOverlap`
  (params (OverlappedComponent :type "PrimitiveComponent Object Reference") (OtherActor :type "Actor Object Reference") (OtherComp :type "PrimitiveComponent Object Reference") (OtherBodyIndex :type Integer) (bFromSweep :type Boolean) (SweepResult :type "HitResult Structure (by ref)"))
  (cast `/Game/Meyer/BP_RotateObjectivePuzzle` OtherActor)
  (set `self.ObjectFourActivate` true))

(event `self.TriggerPuzzleFour.OnComponentEndOverlap`
  (params (OverlappedComponent :type "PrimitiveComponent Object Reference") (OtherActor :type "Actor Object Reference") (OtherComp :type "PrimitiveComponent Object Reference") (OtherBodyIndex :type Integer))
  (cast `/Game/Meyer/BP_RotateObjectivePuzzle` OtherActor)
  (set `self.ObjectFourActivate` false))

(fn `UserConstructionScript`)