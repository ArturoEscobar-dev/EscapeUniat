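; BP_WallDoor is a wall door that opens when enough linked pressure switches are active.
; SwitchActivated and SwitchDesactivated events raise or lower a counter, then compare it to the required switch count.
; Meeting the count plays a timeline that moves the door mesh along its relative Z position; falling short reverses it.
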(event `SwitchActivated`
  (bind _pressureswitchesactive (`self.PressureSwitchesActive`))
  (`/Engine/EditorBlueprintResources/StandardMacros.IncrementInt` _pressureswitchesactive
    (:`  `
      (if (>= _pressureswitchesactive (`self.PressureSwitchesNeeded`))
        (bind (_direction _walldoorposition) (`Timeline|WallDoorAction` :!label _label)
          (:`Update`
            (`SceneComponent.K2_SetRelativeLocation` (`self.WallDoor`) (`KismetMathLibrary.MakeVector` 0.0 0.0 _walldoorposition) false false)))
        (else
          (goto _label :!via `Reverse`))))))

(event `SwitchDesactivated`
  (bind _pressureswitchesactive (`self.PressureSwitchesActive`))
  (`/Engine/EditorBlueprintResources/StandardMacros.DecrementInt` _pressureswitchesactive
    (:`  `
      (if (>= _pressureswitchesactive (`self.PressureSwitchesNeeded`))
        (goto _label)
        (else
          (goto _label :!via `Reverse`))))))

(fn `UserConstructionScript`)