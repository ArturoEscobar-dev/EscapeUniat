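; BP_Door is a hinged door that shows an interact prompt when something overlaps its Box.
; Open_Door alternates through a FlipFlop, playing or reversing a timeline that lerps the door's yaw between closed and a quarter turn open.
; Box overlap begin adds a new P_Interact widget to the viewport.
; Overlap end constructs another unused P_Interact, then clears all widgets, not just the prompt.
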(event `Open_Door`
  (`/Engine/EditorBlueprintResources/StandardMacros.FlipFlop`
    (:`A`
      (bind (_direction _door_float) (`Timeline|Open_DoorT` :!label _label)
        (:`Update`
          (`SceneComponent.K2_SetRelativeRotation` (`self.Door`) (`KismetMathLibrary.MakeRotator` 0.0 0.0 (`KismetMathLibrary.Lerp` 0.0 90.0 _door_float)) false false))))
    (:`B`
      (goto _label :!via `Reverse`))))

(event `self.Box.OnComponentBeginOverlap`
  (params (OverlappedComponent :type "PrimitiveComponent Object Reference") (OtherActor :type "Actor Object Reference") (OtherComp :type "PrimitiveComponent Object Reference") (OtherBodyIndex :type Integer) (bFromSweep :type Boolean) (SweepResult :type "HitResult Structure (by ref)"))
  (bind _returnvalue (`|GenericCreateObject` "/Game/Meyer/P_Interact.P_Interact_C"))
  (bind _output_get (set `self.HUD` _returnvalue))
  (`UserWidget.AddToViewport` _output_get 0))

(event `self.Box.OnComponentEndOverlap`
  (params (OverlappedComponent :type "PrimitiveComponent Object Reference") (OtherActor :type "Actor Object Reference") (OtherComp :type "PrimitiveComponent Object Reference") (OtherBodyIndex :type Integer))
  (bind _returnvalue (`|GenericCreateObject` "/Game/Meyer/P_Interact.P_Interact_C"))
  (set `self.HUD` _returnvalue)
  (`WidgetLayoutLibrary.RemoveAllWidgets`))

(fn `UserConstructionScript`)