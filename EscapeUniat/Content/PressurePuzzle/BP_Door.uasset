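; Door actor for the pressure puzzle that slides from its starting location to an end location over a set time.
; BeginPlay stores the start position, and Tick accumulates elapsed time to lerp the location, using RotationTime as the duration despite the motion being translation.
; Tick switches itself off once that duration is reached.
; The OpenDoors event also disables ticking, so as written it halts movement rather than starting it.
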(event `self.ReceiveBeginPlay`
  (set `self.StartLocation` (`self.K2_GetActorLocation`)))

(event `/Game/PressurePuzzle/PuzzleInterface.OpenDoors`
  (`self.SetActorTickEnabled` false))

(event `self.ReceiveTick`
  (params (DeltaSeconds :type "Float (single-precision)"))
  (set `self.currentTime` (+ DeltaSeconds (`self.currentTime`)))
  (`self.K2_SetActorLocation` (`KismetMathLibrary.VLerp` (`self.StartLocation`) (`self.EndLocation`) (/ (`self.currentTime`) (`self.RotationTime`))))
  (if (>= (`self.currentTime`) (`self.RotationTime`))
    (`self.SetActorTickEnabled` false)))

(fn `UserConstructionScript`)