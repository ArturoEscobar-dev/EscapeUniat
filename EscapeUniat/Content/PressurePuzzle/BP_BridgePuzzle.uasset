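; Bridge puzzle actor where the player rotates three cube components with Z, X, C and V while inside its Box trigger.
; Each key picks one of four preset offsets per cube, turning all three at once and ignoring new presses while moving.
; Tick, enabled on demand, interpolates the turn, then saves the new start rotations.
; When every cube matches CompleteRotation within tolerance, it messages Doors to open.
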(event `self.Box.OnComponentBeginOverlap`
  (params (OverlappedComponent :type "PrimitiveComponent Object Reference") (OtherActor :type "Actor Object Reference") (OtherComp :type "PrimitiveComponent Object Reference") (OtherBodyIndex :type Integer) (bFromSweep :type Boolean) (SweepResult :type "HitResult Structure (by ref)"))
  (cast `/Game/ThirdPerson/Blueprints/BP_ThirdPersonCharacter` OtherActor)
  (`self.EnableInput` (`GameplayStatics.GetPlayerController` 0)))

(event `self.Box.OnComponentEndOverlap`
  (params (OverlappedComponent :type "PrimitiveComponent Object Reference") (OtherActor :type "Actor Object Reference") (OtherComp :type "PrimitiveComponent Object Reference") (OtherBodyIndex :type Integer))
  (cast `/Game/ThirdPerson/Blueprints/BP_ThirdPersonCharacter` OtherActor)
  (`self.DisableInput` (`GameplayStatics.GetPlayerController` 0)))

(event `self.ReceiveBeginPlay`
  (bind _cube3 (`self.Cube3`))
  (bind _cube1 (`self.Cube1`))
  (bind _cube2 (`self.Cube2`))
  (`KismetArrayLibrary.Array_Add` (`self.Data`) (make `/Game/PressurePuzzle/S_PuzzleData` _cube1 (`SceneComponent.RelativeRotation` _cube1) (`|MakeArray` (struct :`Pitch` 10.0) (struct :`Pitch` 25.0) (struct :`Pitch` -30.0) (struct :`Pitch` -15.0) :!type "Rotator Structure")))
  (`KismetArrayLibrary.Array_Add` (`self.Data`) (make `/Game/PressurePuzzle/S_PuzzleData` _cube2 (`SceneComponent.RelativeRotation` _cube2) (`|MakeArray` (struct :`Pitch` 40.0) (struct :`Pitch` 15.0) (struct :`Pitch` -10.0) (struct :`Pitch` -25.0) :!type "Rotator Structure")))
  (`KismetArrayLibrary.Array_Add` (`self.Data`) (make `/Game/PressurePuzzle/S_PuzzleData` _cube3 (`SceneComponent.RelativeRotation` _cube3) (`|MakeArray` (struct :`Pitch` 35.0) (struct :`Pitch` 25.0) (struct :`Pitch` -15.0) (struct :`Pitch` -5.0) :!type "Rotator Structure"))))

(event `Key|Z`
  (params (Key :type "Key Structure"))
  (:`Pressed`
    (`self.TryRotation` 0)))

(event `Key|C`
  (params (Key :type "Key Structure"))
  (:`Pressed`
    (`self.TryRotation` 1)))

(event `Key|X`
  (params (Key :type "Key Structure"))
  (:`Pressed`
    (`self.TryRotation` 2)))

(event `Key|V`
  (params (Key :type "Key Structure"))
  (:`Pressed`
    (`self.TryRotation` 3)))

(event `RotateStuff`
  (bind _returnvalue (/ (`self.CurrentTime`) (`self.RotationTime`)))
  (for _array_element (`self.Data`)
    (bind (_component _startrotation _rotation) (break `/Game/PressurePuzzle/S_PuzzleData` _array_element))
    (bind (_output_roll _output_pitch _output_yaw) (`KismetMathLibrary.BreakRotator` (`|GetArrayItem` _rotation (`self.RotationIndex`))))
    (`SceneComponent.K2_SetRelativeRotation` _component (`KismetMathLibrary.ComposeRotators` _startrotation (`KismetMathLibrary.MakeRotator` (* _output_roll _returnvalue) (* _output_pitch _returnvalue) (* _output_yaw _returnvalue))) false false))
  (if (>= (`self.CurrentTime`) (`self.RotationTime`))
    (set `self.isMoving` false)
    (`self.SetActorTickEnabled` false)
    (set `self.CurrentTime` 0.0)
    (for (_array_element_2 _array_index) (`self.Data`)
      (bind (_component_2 _startrotation_2 _rotation_2) (break `/Game/PressurePuzzle/S_PuzzleData` _array_element_2))
      (bind _returnvalue_2 (`KismetMathLibrary.ComposeRotators` _startrotation_2 (`|GetArrayItem` _rotation_2 (`self.RotationIndex`))))
      (`SceneComponent.K2_SetRelativeRotation` _component_2 _returnvalue_2 false false)
      (bind _structout (setmembers `/Game/PressurePuzzle/S_PuzzleData` :`StructRef` _array_element_2 :`StartRotation` _returnvalue_2))
      (`KismetArrayLibrary.Array_Set` (`self.Data`) _array_index _structout))
    (bind _success (`self.IsPuzzleFinished`))
    (if _success
      (message `/Game/PressurePuzzle/PuzzleInterface.OpenDoors` (`self.Doors`)))))

(event `self.ReceiveTick`
  (params (DeltaSeconds :type "Float (single-precision)"))
  (set `self.CurrentTime` (+ DeltaSeconds (`self.CurrentTime`)))
  (`self.RotateStuff`))

(event `TryRotation`
  (params (RotationIndex :type Integer))
  (if (not (`self.isMoving`))
    (set `self.isMoving` true)
    (set `self.RotationIndex` RotationIndex)
    (`self.SetActorTickEnabled` true)))

(fn `IsPuzzleFinished`
  (returns (Success :type Boolean))
  (locals (L_Success :type Boolean :default true))
  (for (_array_element _array_index) (`self.CompleteRotation`)
    (bind _output_component (break `/Game/PressurePuzzle/S_PuzzleData` (`|GetArrayItem` (`self.Data`) _array_index)))
    (if (not (== (`SceneComponent.RelativeRotation` _output_component) _array_element :`ErrorTolerance` 0.5))
      (set `local.L_Success` false)))
  (return (`local.L_Success`)))

(fn `UserConstructionScript`)