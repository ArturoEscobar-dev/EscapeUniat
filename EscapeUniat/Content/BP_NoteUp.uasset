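; BP_NoteUp is a note pickup that shows its text on screen when the third-person character walks into it.
; Overlapping its box creates a WBI_Note widget, passes it the actor's Text, adds it to the viewport and hides the cube mesh.
; After a three-second delay it removes the widget and destroys itself.
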(event `PickUpNote`
  (bind _returnvalue (`|CreateWidget` "/Game/WBI_Note.WBI_Note_C"))
  (bind _output_get (set `self.NewVar` _returnvalue))
  (`/Game/WBI_Note.Change Number` _output_get (`self.Text`))
  (`UserWidget.AddToViewport` _output_get 0)
  (`SceneComponent.SetVisibility` (`self.Cube`) false false))

(event `PutDownNote`
  (`Widget.RemoveFromParent` (`self.NewVar`)))

(event `self.Box.OnComponentBeginOverlap`
  (params (OverlappedComponent :type "PrimitiveComponent Object Reference") (OtherActor :type "Actor Object Reference") (OtherComp :type "PrimitiveComponent Object Reference") (OtherBodyIndex :type Integer) (bFromSweep :type Boolean) (SweepResult :type "HitResult Structure (by ref)"))
  (cast `/Game/ThirdPerson/Blueprints/BP_ThirdPersonCharacter` OtherActor)
  (`self.PickUpNote`)
  (`KismetSystemLibrary.Delay` 3.0)
  (`self.PutDownNote`)
  (`self.K2_DestroyActor`))

(fn `UserConstructionScript`)