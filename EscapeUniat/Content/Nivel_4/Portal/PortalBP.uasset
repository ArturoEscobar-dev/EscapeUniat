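; PortalBP is a paired portal actor that moves the player character to the ExitReference of another portal sharing its PortalIndex.
; Overlap searches all portals for the opposite Entrada end, disabling both briefly to prevent bouncing; any actor triggers it, as the character cast is disconnected.
; BeginPlay applies material, visibility and Plane removal from flags.
; Scene-capture perspective and construction setup are disconnected, so the per-tick UpdateCamera does nothing.
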(event `self.ReceiveBeginPlay`
  (bind _portal (`self.Portal`))
  (bind _plane (`self.Plane`))
  (if (`self.Camara?`)
    (`PrimitiveComponent.SetMaterial` _portal 0 "/Game/Nivel_4/Portal/Textures/RT_P_MI_2.RT_P_MI_2")
    (else
      (`PrimitiveComponent.SetMaterial` _portal 0 (`self.Material`))))
  (`SceneComponent.SetVisibility` _plane false false)
  (if (not (`self.visible?`))
    (`SceneComponent.SetVisibility` _portal false false)
    (`SceneComponent.SetVisibility` _plane false false))
  (if (not (`self.Collision`))
    (`ActorComponent.K2_DestroyComponent` _plane)))

(event `self.ReceiveActorBeginOverlap`
  (params (OtherActor :type "Actor Object Reference")))

(event `self.ReceiveTick`
  (params (DeltaSeconds :type "Float (single-precision)"))
  (`self.UpdateCamera`))

(event `self.Portal.OnComponentBeginOverlap`
  (params (OverlappedComponent :type "PrimitiveComponent Object Reference") (OtherActor :type "Actor Object Reference") (OtherComp :type "PrimitiveComponent Object Reference") (OtherBodyIndex :type Integer) (bFromSweep :type Boolean) (SweepResult :type "HitResult Structure (by ref)"))
  (bind _returnvalue (`GameplayStatics.GetPlayerCharacter` 0))
  ;[1 0.06771 0.06771] Conectar con otra puerta de teletransporte del mismo tipo y teletransportar
  (if (`self.PuedePasar`)
    (if (`self.CanTeleport?`)
      (if (`self.Entrada`)
        (bind _outactors (`GameplayStatics.GetAllActorsOfClass` "PortalBP_C"))
        (for _array_element _outactors
          (if (and (== (`/Game/Nivel_4/Portal/PortalBP.PortalIndex` _array_element) (`self.PortalIndex`)) (not (`/Game/Nivel_4/Portal/PortalBP.Entrada` _array_element)))
            (break)))
        (set `/Game/Nivel_4/Portal/PortalBP.CanTeleport?` false _array_element)
        (set `self.CanTeleport?` false)
        (`self.K2_SetActorLocation` _returnvalue (`SceneComponent.K2_GetComponentLocation` (`/Game/Nivel_4/Portal/PortalBP.ExitReference` _array_element)) false false)
        (`KismetSystemLibrary.Delay` 0.5)
        (set `/Game/Nivel_4/Portal/PortalBP.CanTeleport?` true _array_element)
        (set `self.CanTeleport?` true)
        (else
          (bind _outactors_2 (`GameplayStatics.GetAllActorsOfClass` "PortalBP_C"))
          (for _array_element_2 _outactors_2
            (if (and (== (`/Game/Nivel_4/Portal/PortalBP.PortalIndex` _array_element_2) (`self.PortalIndex`)) (and (not (`self.Entrada`)) (`/Game/Nivel_4/Portal/PortalBP.Entrada` _array_element_2)))
              (break)))
          (set `/Game/Nivel_4/Portal/PortalBP.CanTeleport?` false _array_element_2)
          (set `self.CanTeleport?` false)
          (`self.K2_SetActorLocation` _returnvalue (`SceneComponent.K2_GetComponentLocation` (`/Game/Nivel_4/Portal/PortalBP.ExitReference` _array_element_2)) false false)
          (`KismetSystemLibrary.Delay` 0.5)
          (set `/Game/Nivel_4/Portal/PortalBP.CanTeleport?` true _array_element_2)
          (set `self.CanTeleport?` true))))))

(event `quitar`)

(fn `UpdateCamera`)

(fn `UserConstructionScript`)