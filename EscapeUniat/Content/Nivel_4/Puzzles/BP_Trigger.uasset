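; BP_Trigger is a Level 4 puzzle trigger that teleports whatever qualifies to the location of a referenced Actor.
; When its Box is overlapped, the Priorizarjugador flag selects the target: only BP_ThirdPersonCharacter if true, otherwise only actors tagged "cubo".
; The teleport replaces the overlapping actor's location while keeping its rotation and scale.
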(event `self.Box.OnComponentBeginOverlap`
  (params (OverlappedComponent :type "PrimitiveComponent Object Reference") (OtherActor :type "Actor Object Reference") (OtherComp :type "PrimitiveComponent Object Reference") (OtherBodyIndex :type Integer) (bFromSweep :type Boolean) (SweepResult :type "HitResult Structure (by ref)"))
  (bind (_returnvalue_location _returnvalue_rotation _returnvalue_scale) (`KismetMathLibrary.BreakTransform` (`self.GetTransform` OtherActor)))
  (if (`self.priorizarjugador?`)
    (bind _asbp_third_person_character (cast `/Game/ThirdPerson/Blueprints/BP_ThirdPersonCharacter` OtherActor))
    (bind (_returnvalue_location_2 _returnvalue_rotation_2 _returnvalue_scale_2) (`KismetMathLibrary.BreakTransform` (`self.GetTransform` _asbp_third_person_character)))
    (`self.K2_SetActorTransform` _asbp_third_person_character (`KismetMathLibrary.MakeTransform` (`self.K2_GetActorLocation` (`self.actor`)) _returnvalue_rotation_2 _returnvalue_scale_2) false false)
    (elif (`self.ActorHasTag` OtherActor "cubo")
      (`self.K2_SetActorTransform` OtherActor (`KismetMathLibrary.MakeTransform` (`self.K2_GetActorLocation` (`self.actor`)) _returnvalue_rotation _returnvalue_scale) false false))))

(fn `UserConstructionScript`)